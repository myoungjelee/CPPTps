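; BP_Only_Bullet is a simple projectile actor that flies straight along its forward vector and expires after a short lifetime.
; Tick offsets its location by Speed scaled by delta time, without sweeping for collision.
; BeginPlay starts a timer that calls Die to destroy the actor after two seconds.
; It contains no hit or damage logic, as the overlap event is an unused disabled stub.
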(event `self.ReceiveBeginPlay`
  (`KismetSystemLibrary.K2_SetTimer` null "Die" 2.0))

(event `self.ReceiveTick`
  (params (DeltaSeconds :type "Float (single-precision)"))
  (`self.K2_SetActorLocation` (+ (`self.K2_GetActorLocation`) (* DeltaSeconds (* (`self.GetActorForwardVector`) (`self.Speed`))))))

(fn `Die`
  (`self.K2_DestroyActor`))

(fn `UserConstructionScript`)