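; Enemy AI state machine component that drives a BP_Only_Enemy through idle, move, attack, attack delay, damaged and die states.
; Tick runs the current state; ChangeState stops movement, syncs the anim Blueprint and plays damage or death montages.
; A view-cone and line-trace check switches between chasing the player and roaming to random navmesh points.
; ReceiveDamage decrements HP; dead enemies sink once Dying is set, then return to BP_Only_EnemyManager's pool.
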(event `self.ReceiveBeginPlay`
  ;[1 1 1] 타겟(플레이어)를 찾자
  (bind _returnvalue (`GameplayStatics.GetActorOfClass` "/Game/Blueprints/Only/BP_Only_TpsPlayer.BP_Only_TpsPlayer_C"))
  (set `self.Player` _returnvalue)
  ;[1 1 1] 나를 찾자
  (bind _asbp_only_enemy (cast `/Game/Blueprints/Only/BP_Only_Enemy` (`self.GetOwner`)))
  (set `self.Me` _asbp_only_enemy)
  (set `self.HP` (`self.InitialHP`))
  ;[1 1 1] 애니메이션 블루프린트 가져오기
  (bind _asabp_only_enemy (cast `/Game/Blueprints/Only/ABP_Only_Enemy` (`SkeletalMeshComponent.GetAnimInstance` (`Character.Mesh` (`self.Me`)))))
  (set `self.Anim` _asabp_only_enemy)
  (set `self.AI` (`AIBlueprintHelperLibrary.GetAIController` (`self.Me`))))

(event `self.ReceiveTick`
  (params (DeltaSeconds :type "Float (single-precision)"))
  (switch `/Game/Blueprints/Only/Bp_EnemyState` (`self.State`)
    (:`NewEnumerator0`
      (`self.Idle`))
    (:`NewEnumerator1`
      (`self.Move`))
    (:`NewEnumerator2`
      (`self.Attack`))
    (:`NewEnumerator3`
      (`self.Damaged`))
    (:`NewEnumerator4`
      (`self.Die`))
    (:`NewEnumerator5`
      (`self.AttackDelay`))))

(fn `Attack`
  (`self.ChangeState` "NewEnumerator5"))

(fn `AttackDelay`
  (bind _complete (`self.FlowTime` (`self.AttackDelayTime`)))
  (if _complete
    (if (< (`KismetMathLibrary.VSize` (- (`Actor.K2_GetActorLocation` (`self.Player`)) (`Actor.K2_GetActorLocation` (`self.Me`)))) (`self.AttackRange`))
      (`self.ChangeState` "NewEnumerator2")
      (else
        (`self.ChangeState` "NewEnumerator0")))))

(fn `ChangeState`
  (params (s :type "/Game/Blueprints/Only/Bp_EnemyState Enum" :default "NewEnumerator0"))
  (set `self.CurrTime` 0.0)
  (`Controller.StopMovement` (`self.AI`))
  (bind _output_get (set `self.State` s))
  (bind _output_get_2 (set `/Game/Blueprints/Only/ABP_Only_Enemy.State` _output_get (`self.Anim`)))
  (switch `/Game/Blueprints/Only/Bp_EnemyState` _output_get_2
    (:`NewEnumerator1`
      (set `self.RandPos` (`NavigationSystemV1.K2_GetRandomReachablePointInRadius` (`NavigationSystemV1.GetNavigationSystem`) (`Actor.K2_GetActorLocation` (`self.Me`)) 10000.0 null null)))
    (:`NewEnumerator3`
      (`Character.PlayAnimMontage` (`self.Me`) "/Game/Blueprints/AMT_Enemy_Damage.AMT_Enemy_Damage" 1.0 (`KismetStringLibrary.Conv_StringToName` (`KismetStringLibrary.Concat_StrStr` "Damage" (`KismetStringLibrary.Conv_IntToString` (`KismetMathLibrary.RandomIntegerInRange` 0 1))))))
    (:`NewEnumerator4`
      (`PrimitiveComponent.SetCollisionEnabled` (`Character.CapsuleComponent` (`self.Me`)) "NoCollision")
      (`Character.PlayAnimMontage` (`self.Me`) "/Game/Blueprints/AMT_Enemy_Damage.AMT_Enemy_Damage" 1.0 "Die"))))

(fn `Damaged`
  (bind _complete (`self.FlowTime` (`self.DamagedDelayTime`)))
  (if _complete
    (`self.ChangeState` "NewEnumerator1")))

(fn `Die`
  (bind _me (`self.Me`))
  (bind (_returnvalue_x _returnvalue_y _returnvalue_z) (`KismetMathLibrary.BreakVector` (`Actor.K2_GetActorLocation` (`self.Me`))))
  (if (`self.Dying`)
    (`Actor.K2_SetActorLocation` _me (+ (`Actor.K2_GetActorLocation` _me) (* (* (`KismetMathLibrary.Vector_Down`) (`self.DieSpeed`)) (`GameplayStatics.GetWorldDeltaSeconds`))) false false)
    (if (< _returnvalue_z -200.0)
      (`/Game/Blueprints/Only/BP_Only_Enemy.SetActive` (`self.Me`) false)
      (bind _returnvalue (`GameplayStatics.GetActorOfClass` "/Game/Blueprints/Only/BP_Only_EnemyManager.BP_Only_EnemyManager_C"))
      (`KismetArrayLibrary.Array_Add` (`/Game/Blueprints/Only/BP_Only_EnemyManager.enemyArray` _returnvalue) (`self.Me`))
      (set `self.HP` (`self.InitialHP`))
      (`self.ChangeState` "NewEnumerator0")
      (`Character.StopAnimMontage` (`self.Me`) "/Game/Blueprints/AMT_Enemy_Damage.AMT_Enemy_Damage")
      (set `self.Dying` false))))

(fn `FlowTime`
  (params (`Delay Time` :type "Float (double-precision)"))
  (returns (Complete :type Boolean))
  (bind _output_get (set `self.CurrTime` (+ (`GameplayStatics.GetWorldDeltaSeconds`) (`self.CurrTime`))))
  (if (== (> _output_get `Delay Time`) true)
    (set `self.CurrTime` 0.0)
    (return true)
    (else
      (return false))))

(fn `Idle`
  (bind _btrace (`self.IsTargetTrace`))
  (if _btrace
    (`self.ChangeState` "NewEnumerator1")
    (else
      (bind _complete (`self.FlowTime` (`self.IdleDelayTime`)))
      (if _complete
        (`self.ChangeState` "NewEnumerator1")))))

(fn `IsTargetTrace`
  (returns (bTrace :type Boolean))
  (if (< (`KismetMathLibrary.DegAcos` (`KismetMathLibrary.Dot_VectorVector` (`Actor.GetActorForwardVector` (`self.Me`)) (`KismetMathLibrary.Normal` (- (`Actor.K2_GetActorLocation` (`self.Player`)) (`Actor.K2_GetActorLocation` (`self.Me`)))))) 30.0)
    (bind _outhit (`KismetSystemLibrary.LineTraceSingle` (`Actor.K2_GetActorLocation` (`self.Me`)) (`Actor.K2_GetActorLocation` (`self.Player`)) "TraceTypeQuery1"))
    (return (`KismetStringLibrary.Contains` (`KismetSystemLibrary.GetDisplayName` (`.HitActor` (`GameplayStatics.BreakHitResult` _outhit))) "Player"))
    (else
      (return false))))

(fn `Move`
  (bind _btrace (`self.IsTargetTrace`))
  (if _btrace
    ;[1 1 1] 시야에 들어왔을때 행동
    (if (< (`KismetMathLibrary.VSize` (- (`Actor.K2_GetActorLocation` (`self.Player`)) (`Actor.K2_GetActorLocation` (`self.Me`)))) (`self.AttackRange`))
      (`self.ChangeState` "NewEnumerator2")
      (else
        (`AIController.MoveToLocation` (`self.AI`) (`Actor.K2_GetActorLocation` (`self.Player`)) -1.0 true true false true null true)))
    (else
      ;[1 1 1] 시야에 안들어왔을때 ㅎ애동
      (bind _returnvalue (`AIController.MoveToLocation` (`self.AI`) (`self.RandPos`) -1.0 true true false true null true))
      (if (`|EnumEquality` _returnvalue "AlreadyAtGoal")
        (`self.ChangeState` "NewEnumerator0")))))

(fn `ReceiveDamage`
  (bind _output_get (set `self.HP` (- (`self.HP`) 1.0)))
  (if (> _output_get 0.0)
    (`self.ChangeState` "NewEnumerator3")
    (else
      (`self.ChangeState` "NewEnumerator4"))))