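; BP_Only_Enemy is an enemy character whose behavior component is BPOnlyEnemyFSM, apparently a state machine.
; On BeginPlay it sets character movement to orient rotation toward the movement direction.
; SetActive switches the enemy on or off as a whole without destroying it, toggling mesh activity and visibility, movement, the FSM and capsule collision together.
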(event `self.ReceiveBeginPlay`
  (set `CharacterMovementComponent.bOrientRotationToMovement` true (`self.CharacterMovement`)))

(event `self.ReceiveTick`
  (params (DeltaSeconds :type "Float (single-precision)")))

(fn `SetActive`
  (params (bActive :type Boolean))
  (bind _mesh (`self.Mesh`))
  (bind _capsulecomponent (`self.CapsuleComponent`))
  (`ActorComponent.SetActive` _mesh bActive false)
  (`SceneComponent.SetVisibility` _mesh bActive false)
  (`ActorComponent.SetActive` (`self.CharacterMovement`) bActive false)
  (`ActorComponent.SetActive` (`self.BP_Only_EnemyFSM`) bActive false)
  (if bActive
    (`PrimitiveComponent.SetCollisionEnabled` _capsulecomponent "QueryAndPhysics")
    (else
      (`PrimitiveComponent.SetCollisionEnabled` _capsulecomponent "NoCollision"))))

(fn `UserConstructionScript`)