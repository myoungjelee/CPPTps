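; BP_Only_EnemyManager spawns a small, inactive pool of BP_Only_Enemy actors at BeginPlay and releases them over time.
; Tick waits a random interval, then positions and activates the first pooled enemy and removes it from the array.
; Placement cycles through the level's BP_SpawnPos actors, randomly yawing each to place the enemy at a random distance along its forward vector, facing that direction.
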(event `self.ReceiveBeginPlay`
  (set `self.makeTime` (`KismetMathLibrary.RandomFloatInRange` (`self.minTime`) (`self.maxTime`)))
  (bind _outactors (`GameplayStatics.GetAllActorsOfClass` "/Game/Blueprints/BP_SpawnPos.BP_SpawnPos_C"))
  (set `self.spawnPosArray` _outactors)
  (for _ (range 3)
    (bind _returnvalue (`|SpawnActorFromClass` "/Game/Blueprints/Only/BP_Only_Enemy.BP_Only_Enemy_C" (`self.GetTransform`) "AlwaysSpawn" "OverrideRootScale" null null))
    (`KismetArrayLibrary.Array_Add` (`self.enemyArray`) _returnvalue)
    (`/Game/Blueprints/Only/BP_Only_Enemy.SetActive` _returnvalue false)))

(event `self.ReceiveTick`
  (params (DeltaSeconds :type "Float (single-precision)"))
  (bind _output (`|GetArrayItem` (`self.enemyArray`)))
  (if (not (== (`KismetArrayLibrary.Array_Length` (`self.enemyArray`)) 0))
    (bind _output_get (set `self.currTime` (+ DeltaSeconds (`self.currTime`))))
    (if (> _output_get (`self.makeTime`))
      (bind (_output_2 _returnvalue) (`self.RotationPos`))
      (`self.K2_SetActorLocationAndRotation` _output _returnvalue (`self.K2_GetActorRotation` _output_2) false false)
      (`/Game/Blueprints/Only/BP_Only_Enemy.SetActive` _output true)
      (`KismetArrayLibrary.Array_Remove` (`self.enemyArray`))
      (set `self.currTime` 0.0)
      (set `self.makeTime` (`KismetMathLibrary.RandomFloatInRange` (`self.minTime`) (`self.maxTime`)))
      (bind _result (`/Engine/EditorBlueprintResources/StandardMacros.IncrementInt` (`self.spawnIdx`))
        (:`  `
          (if (== _result (`KismetArrayLibrary.Array_Length` (`self.spawnPosArray`)))
            (set `self.spawnIdx` 0)))))))

(fn `RotationPos`
  (returns (Output :type "Actor Object Reference") (ReturnValue :type "Vector Structure"))
  (bind _output (`|GetArrayItem` (`self.spawnPosArray`) (`self.spawnIdx`)))
  (`self.K2_SetActorRotation` _output (`KismetMathLibrary.MakeRotator` 0.0 0.0 (`KismetMathLibrary.RandomFloatInRange` 0.0 360.0)) false)
  (return _output (+ (`self.K2_GetActorLocation` _output) (* (`self.GetActorForwardVector` _output) (`KismetMathLibrary.RandomFloatInRange` 300.0 1000.0)))))

(fn `UserConstructionScript`)